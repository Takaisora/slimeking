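; AI slime pawn linked to player 2 that any of the four player characters absorbs on overlap, gaining split-slime score before it destroys itself.
; Pawn sensing writes a seen BP_Character_02 to the blackboard's Player key.
; It also carries player-style functions, uncalled here: score gains that rescale the mesh and update GameInstance's Slime2Score, plus Wolf, Wisp and WingRabbit ability pickup and effects, several hard-wired to player character indices.
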(event `self.PawnSensing1.OnSeePawn`
  (params (Pawn :type "Pawn Object Reference"))
  (bind _asbp_character_02 (cast `/Game/BluePrints/BP_Character/BP_Character_02` Pawn))
  (`BlackboardComponent.SetValueAsObject` (`AIBlueprintHelperLibrary.GetBlackboard` self) "Player" _asbp_character_02))

(event `self.Sphere.OnComponentBeginOverlap`
  (params (OverlappedComponent :type "PrimitiveComponent Object Reference") (OtherActor :type "Actor Object Reference") (OtherComp :type "PrimitiveComponent Object Reference") (OtherBodyIndex :type Integer) (bFromSweep :type Boolean) (SweepResult :type "HitResult Structure (by ref)"))
  (bind (_asbp_character_02 _bsuccess) (cast `/Game/BluePrints/BP_Character/BP_Character_02` OtherActor :!pure true))
  (bind (_asbp_character _bsuccess_2) (cast `/Game/BluePrints/BP_Character/BP_Character` OtherActor :!pure true))
  (bind (_asbp_character_03 _bsuccess_3) (cast `/Game/BluePrints/BP_Character/BP_Character_03` OtherActor :!pure true))
  (bind (_asbp_character_04 _bsuccess_4) (cast `/Game/BluePrints/BP_Character/BP_Character_04` OtherActor :!pure true))
  (`|ExecutionSequence`
    (:`then_0`
      (if _bsuccess
        (`/Game/BluePrints/BP_Character/BP_Character_02.AddScoreSplitSlime` _asbp_character_02)
        (`self.K2_DestroyActor` :!label _label)))
    (:`then_1`
      (if _bsuccess_2
        (`/Game/BluePrints/BP_Character/BP_Character.AddScoreSplitSlime` _asbp_character)
        (goto _label)))
    (:`then_2`
      (if _bsuccess_3
        (`/Game/BluePrints/BP_Character/BP_Character_03.AddScoreSplitSlime` _asbp_character_03)
        (goto _label)))
    (:`then_3`
      (if _bsuccess_4
        (`/Game/BluePrints/BP_Character/BP_Character_04.AddScoreSplitSlime` _asbp_character_04)
        (goto _label)))))

(fn `AbilityJumpSteta`
  (set `CharacterMovementComponent.JumpZVelocity` 800.0 (`self.CharacterMovement`)))

(fn `AbilityWalkSpeed`
  (set `CharacterMovementComponent.MaxWalkSpeed` 600.0 (`self.CharacterMovement`)))

(fn `AddItem`
  (bind _actortrace (`self.ActorTrace`))
  (bind _actortrace_2 (`self.ActorTrace`))
  (bind (_asbp_wolf _bsuccess) (cast `/Game/Enemy/Wolf/BP_Wolf` _actortrace_2 :!pure true))
  (bind (_asbp_wolf_2 _bsuccess_2) (cast `/Game/Enemy/Wolf/BP_Wolf` _actortrace :!pure true))
  (bind (_asbp_whisp _bsuccess_3) (cast `/Game/Enemy/Whisp/BP_Whisp` _actortrace :!pure true))
  (bind (_asbp_whisp_2 _bsuccess_4) (cast `/Game/Enemy/Whisp/BP_Whisp` _actortrace_2 :!pure true))
  (bind (_asbp_wing_rabbit _bsuccess_5) (cast `/Game/Enemy/WingRabbit/BP_WingRabbit` _actortrace :!pure true))
  (bind (_asbp_wing_rabbit_2 _bsuccess_6) (cast `/Game/Enemy/WingRabbit/BP_WingRabbit` _actortrace_2 :!pure true))
  (`GameplayStatics.PlaySoundAtLocation` null (0.0 0.0 0.0) (struct) 1.0 1.0 0.0 "/Game/Sounds/NewSoundAttenuation.NewSoundAttenuation" null null) ; Acquired Ability
  (if (`self.HaveItem?`)
    (set `self.WolfAbirity2` false)
    (set `self.WispAbility2` false)
    (set `self.WingRabbitAbility` false)
    (`|ExecutionSequence`
      (:`then_0`
        (if _bsuccess_2
          (`KismetArrayLibrary.Array_Add` (`self.Inventory`) (`/Game/BluePrints/BP_Inventory/Inventory/test.ItemData` _asbp_wolf_2))
          (if _bsuccess_2
            (set `self.WolfAbirity2` true)
            (set `self.HaveItem?` true :!label _label)
            (return))))
      (:`then_1`
        (if _bsuccess_3
          (`KismetArrayLibrary.Array_Add` (`self.Inventory`) (`/Game/BluePrints/BP_Inventory/Inventory/test.ItemData` _asbp_whisp))
          (if _bsuccess_3
            (set `self.WispAbility2` true)
            (goto _label))))
      (:`then_2`
        (if _bsuccess_5
          (`KismetArrayLibrary.Array_Add` (`self.Inventory`) (`/Game/BluePrints/BP_Inventory/Inventory/test.ItemData` _asbp_wing_rabbit))
          (if _bsuccess_5
            (set `self.WingRabbitAbility` true)
            (goto _label)))))
    (else
      (`|ExecutionSequence`
        (:`then_0`
          (if _bsuccess
            (`KismetArrayLibrary.Array_Add` (`self.Inventory`) (`/Game/BluePrints/BP_Inventory/Inventory/test.ItemData` _asbp_wolf))
            (if _bsuccess
              (set `self.WolfAbirity2` true)
              (set `self.HaveItem?` true :!label _label_2)
              (return))))
        (:`then_1`
          (if _bsuccess_4
            (`KismetArrayLibrary.Array_Add` (`self.Inventory`) (`/Game/BluePrints/BP_Inventory/Inventory/test.ItemData` _asbp_whisp_2))
            (if _bsuccess_4
              (set `self.WispAbility2` true)
              (goto _label_2))))
        (:`then_2`
          (if _bsuccess_6
            (`KismetArrayLibrary.Array_Add` (`self.Inventory`) (`/Game/BluePrints/BP_Inventory/Inventory/test.ItemData` _asbp_wing_rabbit_2))
            (if _bsuccess_6
              (set `self.WingRabbitAbility` true)
              (goto _label_2))))))))

(fn `AddScore`
  (bind _output_get (set `self.Score` (+ (`self.Score`) (`self.score_grass_2`))))
  (`SceneComponent.SetWorldScale3D` (`self.Mesh`) (+ (`self.magnification_vector_2`) (* (/ _output_get (`self.magnification_score_2`)) (`self.magnification_2`))))
  (bind _asgame_instace_bp (cast `/Game/BluePrints/BP_Instance/GameInstace_BP` (`GameplayStatics.GetGameInstance`)))
  (set `/Game/BluePrints/BP_Instance/GameInstace_BP.slime_2_score` (`self.Score`) _asgame_instace_bp))

(fn `AddScore_Wolf`
  (bind _output_get (set `self.Score` (+ (`self.Score`) (`self.score_wolf_2`))))
  (`SceneComponent.SetWorldScale3D` (`self.Mesh`) (+ (`self.magnification_vector_2`) (* (/ _output_get (`self.magnification_score_2`)) (`self.magnification_2`))))
  (bind _asgame_instace_bp (cast `/Game/BluePrints/BP_Instance/GameInstace_BP` (`GameplayStatics.GetGameInstance`)))
  (set `/Game/BluePrints/BP_Instance/GameInstace_BP.slime_2_score` (`self.Score`) _asgame_instace_bp)
  (`GameplayStatics.PlaySoundAtLocation` "/Game/Sounds/03_Slime_Acquired.03_Slime_Acquired" (`self.K2_GetActorLocation` (`GameplayStatics.GetPlayerCharacter` 1)) (struct) 1.0 1.0 0.0 "/Game/Sounds/NewSoundAttenuation.NewSoundAttenuation" null null))

(fn `AddScoreLizard`
  (bind _output_get (set `self.Score` (+ (`self.Score`) (`self.ScoreLizard`))))
  (`SceneComponent.SetWorldScale3D` (`self.Mesh`) (+ (`self.magnification_vector_2`) (* (/ _output_get (`self.magnification_score_2`)) (`self.magnification_2`))))
  (bind _asgame_instace_bp (cast `/Game/BluePrints/BP_Instance/GameInstace_BP` (`GameplayStatics.GetGameInstance`)))
  (set `/Game/BluePrints/BP_Instance/GameInstace_BP.slime_2_score` (`self.Score`) _asgame_instace_bp))

(fn `AddScoreWingRabbit`
  (bind _output_get (set `self.Score` (+ (`self.Score`) (`self.Score_WingRabbitt`))))
  (`SceneComponent.SetWorldScale3D` (`self.Mesh`) (+ (`self.magnification_vector_2`) (* (/ _output_get (`self.magnification_score_2`)) (`self.magnification_2`))))
  (bind _asgame_instace_bp (cast `/Game/BluePrints/BP_Instance/GameInstace_BP` (`GameplayStatics.GetGameInstance`)))
  (set `/Game/BluePrints/BP_Instance/GameInstace_BP.slime_2_score` (`self.Score`) _asgame_instace_bp)
  (`GameplayStatics.PlaySoundAtLocation` "/Game/Sounds/03_Slime_Acquired.03_Slime_Acquired" (`self.K2_GetActorLocation` (`GameplayStatics.GetPlayerCharacter` 1)) (struct) 1.0 1.0 0.0 "/Game/Sounds/NewSoundAttenuation.NewSoundAttenuation" null null))

(fn `AddScoreWisp`
  (bind _output_get (set `self.ScoreWisp2` (+ (`self.Score`) (`self.ScoreWisp2`))))
  (`SceneComponent.SetWorldScale3D` (`self.Mesh`) (+ (`self.magnification_vector_2`) (* (/ _output_get (`self.magnification_score_2`)) (`self.magnification_2`))))
  (bind _asgame_instace_bp (cast `/Game/BluePrints/BP_Instance/GameInstace_BP` (`GameplayStatics.GetGameInstance`)))
  (set `/Game/BluePrints/BP_Instance/GameInstace_BP.slime_2_score` (`self.Score`) _asgame_instace_bp)
  (`GameplayStatics.PlaySoundAtLocation` "/Game/Sounds/03_Slime_Acquired.03_Slime_Acquired" (`self.K2_GetActorLocation` (`GameplayStatics.GetPlayerCharacter` 1)) (struct) 1.0 1.0 0.0 "/Game/Sounds/NewSoundAttenuation.NewSoundAttenuation" null null))

(fn `JumpUseScore`
  (set `self.Score` (- (`self.Score`) (`self.JumoScore`))))

(fn `SetWingRabbit`
  (set `CharacterMovementComponent.JumpZVelocity` 1600.0 (`self.CharacterMovement`))
  (`self.Jump` (`GameplayStatics.GetPlayerCharacter` 1)))

(fn `SetWisp`
  (`GameplayStatics.SpawnEmitterAtLocation` "/Game/Perticle/WhispParticle1.WhispParticle1" (`SceneComponent.K2_GetComponentLocation` (`/Game/BluePrints/BP_Character/BP_Character.Camera` (cast `/Game/BluePrints/BP_Character/BP_Character` (`GameplayStatics.GetPlayerCharacter` 0) :!pure true)))))

(fn `SetWolf`
  (set `CharacterMovementComponent.MaxWalkSpeed` 1500.0 (`self.CharacterMovement`))
  (return))

(fn `UserConstructionScript`)

(fn `WingRabbitAbilitySounds`
  (`GameplayStatics.PlaySoundAtLocation` "/Game/Sounds/14_SlimeWing_Descent.14_SlimeWing_Descent" (`self.K2_GetActorLocation` (`GameplayStatics.GetPlayerCharacter` 1)) (struct) 1.0 1.0 0.0 "/Game/Sounds/NewSoundAttenuation.NewSoundAttenuation" null null))