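; Tutorial lizard actor that one of four tutorial player characters collects by touching it once their score is at least 10.
; On static mesh overlap, a sequence tries each character class, checking score and cast success, then calls that character's AddScore and destroys the lizard.
; Two helper functions call AddScoreLizard on the non-tutorial characters of players 0 and 1, but nothing in this graph calls them.
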(event `self.ReceiveBeginPlay`)

(event `self.ReceiveTick`
  (params (DeltaSeconds :type "Float (single-precision)")))

(event `self.StaticMesh.OnComponentBeginOverlap`
  (params (OverlappedComponent :type "PrimitiveComponent Object Reference") (OtherActor :type "Actor Object Reference") (OtherComp :type "PrimitiveComponent Object Reference") (OtherBodyIndex :type Integer) (bFromSweep :type Boolean) (SweepResult :type "HitResult Structure (by ref)"))
  (bind (_asbp_character_turtrial _bsuccess) (cast `/Game/BluePrints/BP_Character/Turtorial/BP_Character_turtrial` OtherActor :!pure true))
  (bind (_asbp_character_02_turtorial _bsuccess_2) (cast `/Game/BluePrints/BP_Character/Turtorial/BP_Character_02_Turtorial` OtherActor :!pure true))
  (bind (_asbp_character_03_turtorial _bsuccess_3) (cast `/Game/BluePrints/BP_Character/Turtorial/BP_Character_03_Turtorial` OtherActor :!pure true))
  (bind (_asbp_character_04_turtorial _bsuccess_4) (cast `/Game/BluePrints/BP_Character/Turtorial/BP_Character_04_Turtorial` OtherActor :!pure true))
  (`|ExecutionSequence`
    (:`then_0`
      (if (>= (`/Game/BluePrints/BP_Character/Turtorial/BP_Character_turtrial.Score` _asbp_character_turtrial) 10)
        (if _bsuccess
          (`/Game/BluePrints/BP_Character/Turtorial/BP_Character_turtrial.AddScore` _asbp_character_turtrial)
          (`self.K2_DestroyActor` :!label _label))))
    (:`then_1`
      (if (>= (`/Game/BluePrints/BP_Character/Turtorial/BP_Character_02_Turtorial.Score` _asbp_character_02_turtorial) 10)
        (if _bsuccess_2
          (`/Game/BluePrints/BP_Character/Turtorial/BP_Character_02_Turtorial.AddScore` _asbp_character_02_turtorial)
          (goto _label))))
    (:`then_2`
      (if (>= (`/Game/BluePrints/BP_Character/Turtorial/BP_Character_03_Turtorial.Score` _asbp_character_03_turtorial) 10)
        (if _bsuccess_3
          (`/Game/BluePrints/BP_Character/Turtorial/BP_Character_03_Turtorial.AddScore` _asbp_character_03_turtorial)
          (goto _label))))
    (:`then_3`
      (if (>= (`/Game/BluePrints/BP_Character/Turtorial/BP_Character_04_Turtorial.Score` _asbp_character_04_turtorial) 10)
        (if _bsuccess_4
          (`/Game/BluePrints/BP_Character/Turtorial/BP_Character_04_Turtorial.AddScore` _asbp_character_04_turtorial)
          (goto _label))))))

(fn `LizardScoreBP1`
  (bind _asbp_character (cast `/Game/BluePrints/BP_Character/BP_Character` (`GameplayStatics.GetPlayerCharacter` 0)))
  (`/Game/BluePrints/BP_Character/BP_Character.AddScoreLizard` _asbp_character null))

(fn `LizardScoreBP2`
  (bind _asbp_character_02 (cast `/Game/BluePrints/BP_Character/BP_Character_02` (`GameplayStatics.GetPlayerCharacter` 1)))
  (`/Game/BluePrints/BP_Character/BP_Character_02.AddScoreLizard` _asbp_character_02 null))

(fn `UserConstructionScript`)