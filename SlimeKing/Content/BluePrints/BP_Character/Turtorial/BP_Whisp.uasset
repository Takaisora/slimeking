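; Tutorial wisp pickup that grants a wisp ability to whichever of four tutorial player characters touches it with enough score.
; A timeline moves the mesh vertically from BeginPlay, and Tick spawns a particle emitter at the mesh every frame.
; Sphere overlap casts to each character, resets its abilities, sets the wisp flag, calls AddScore and destroys the pickup.
; It also shows that character's widget and records the pickup in the game instance.
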(event `self.ReceiveBeginPlay`
  (bind (_direction _z) (`Timeline|move_z`)
    (:`Update`
      (`SceneComponent.K2_AddLocalOffset` (`self.Mesh`) (`KismetMathLibrary.MakeVector` 0.0 0.0 _z) false false))))

(event `self.ReceiveTick`
  (params (DeltaSeconds :type "Float (single-precision)"))
  (`GameplayStatics.SpawnEmitterAtLocation` "/Game/Enemy/Whisp/WhispParticle.WhispParticle" (`SceneComponent.K2_GetComponentLocation` (`self.Mesh`)) (struct) (0.5 0.5 0.5)))

(event `self.Sphere.OnComponentBeginOverlap`
  (params (OverlappedComponent :type "PrimitiveComponent Object Reference") (OtherActor :type "Actor Object Reference") (OtherComp :type "PrimitiveComponent Object Reference") (OtherBodyIndex :type Integer) (bFromSweep :type Boolean) (SweepResult :type "HitResult Structure (by ref)"))
  (bind (_asbp_character_turtrial _bsuccess) (cast `/Game/BluePrints/BP_Character/Turtorial/BP_Character_turtrial` OtherActor :!pure true))
  (bind (_asbp_character_02_turtorial _bsuccess_2) (cast `/Game/BluePrints/BP_Character/Turtorial/BP_Character_02_Turtorial` OtherActor :!pure true))
  (bind (_asbp_character_03_turtorial _bsuccess_3) (cast `/Game/BluePrints/BP_Character/Turtorial/BP_Character_03_Turtorial` OtherActor :!pure true))
  (bind (_asbp_character_04_turtorial _bsuccess_4) (cast `/Game/BluePrints/BP_Character/Turtorial/BP_Character_04_Turtorial` OtherActor :!pure true))
  (`|ExecutionSequence`
    (:`then_0`
      (if _bsuccess
        (if (>= (`/Game/BluePrints/BP_Character/Turtorial/BP_Character_turtrial.Score` _asbp_character_turtrial) 20)
          (`/Game/BluePrints/BP_Character/Turtorial/BP_Character_turtrial.AbilityRisset` _asbp_character_turtrial)
          (set `/Game/BluePrints/BP_Character/Turtorial/BP_Character_turtrial.WispAbility` true _asbp_character_turtrial)
          (`/Game/BluePrints/BP_Character/Turtorial/BP_Character_turtrial.AddScore` _asbp_character_turtrial)
          (`self.K2_DestroyActor`)
          (bind _returnvalue (`|CreateWidget` "/Game/BluePrints/BP_Wiedget/Turtorial/BP1/BP1Wisp.BP1Wisp_C"))
          (`UserWidget.AddToViewport` _returnvalue 0)
          (set `/Game/BluePrints/BP_Instance/GameInstace_BP.BP1Wisp` true (cast `/Game/BluePrints/BP_Instance/GameInstace_BP` (`GameplayStatics.GetGameInstance`) :!pure true)))))
    (:`then_1`
      (if _bsuccess_2
        (if (>= (`/Game/BluePrints/BP_Character/Turtorial/BP_Character_02_Turtorial.Score` _asbp_character_02_turtorial) 20)
          (`/Game/BluePrints/BP_Character/Turtorial/BP_Character_02_Turtorial.AbilityRisset` _asbp_character_02_turtorial)
          (set `/Game/BluePrints/BP_Character/Turtorial/BP_Character_02_Turtorial.WispAbility2` true _asbp_character_02_turtorial)
          (`/Game/BluePrints/BP_Character/Turtorial/BP_Character_02_Turtorial.AddScore` _asbp_character_02_turtorial)
          (`self.K2_DestroyActor`)
          (bind _returnvalue_2 (`|CreateWidget` "/Game/BluePrints/BP_Wiedget/Turtorial/BP2/BP2Wisp.BP2Wisp_C"))
          (`UserWidget.AddToViewport` _returnvalue_2 0)
          (set `/Game/BluePrints/BP_Instance/GameInstace_BP.BP2wisp` true (cast `/Game/BluePrints/BP_Instance/GameInstace_BP` (`GameplayStatics.GetGameInstance`) :!pure true)))))
    (:`then_2`
      (if _bsuccess_3
        (if (>= (`/Game/BluePrints/BP_Character/Turtorial/BP_Character_03_Turtorial.Score` _asbp_character_03_turtorial) 20)
          (`/Game/BluePrints/BP_Character/Turtorial/BP_Character_03_Turtorial.AbilityRisset` _asbp_character_03_turtorial)
          (set `/Game/BluePrints/BP_Character/Turtorial/BP_Character_03_Turtorial.WispAbility` true _asbp_character_03_turtorial)
          (`/Game/BluePrints/BP_Character/Turtorial/BP_Character_03_Turtorial.AddScore` _asbp_character_03_turtorial)
          (`self.K2_DestroyActor`)
          (bind _returnvalue_3 (`|CreateWidget` "/Game/BluePrints/BP_Wiedget/Turtorial/BP3/BP3Wisp.BP3Wisp_C"))
          (`UserWidget.AddToViewport` _returnvalue_3 0)
          (set `/Game/BluePrints/BP_Instance/GameInstace_BP.BP3Wisp` true (cast `/Game/BluePrints/BP_Instance/GameInstace_BP` (`GameplayStatics.GetGameInstance`) :!pure true)))))
    (:`then_3`
      (if _bsuccess_4
        (if (>= (`/Game/BluePrints/BP_Character/Turtorial/BP_Character_04_Turtorial.Score` _asbp_character_04_turtorial) 20)
          (`/Game/BluePrints/BP_Character/Turtorial/BP_Character_04_Turtorial.AbilityRisset` _asbp_character_04_turtorial)
          (set `/Game/BluePrints/BP_Character/Turtorial/BP_Character_04_Turtorial.WispAbility` true _asbp_character_04_turtorial)
          (`/Game/BluePrints/BP_Character/Turtorial/BP_Character_04_Turtorial.AddScore` _asbp_character_04_turtorial)
          (`self.K2_DestroyActor`)
          (bind _returnvalue_4 (`|CreateWidget` "/Game/BluePrints/BP_Wiedget/Turtorial/BP4/BP4Wisp.BP4Wisp_C"))
          (`UserWidget.AddToViewport` _returnvalue_4 0)
          (set `/Game/BluePrints/BP_Instance/GameInstace_BP.BP4Wisp` true (cast `/Game/BluePrints/BP_Instance/GameInstace_BP` (`GameplayStatics.GetGameInstance`) :!pure true)))))))

(fn `UserConstructionScript`)