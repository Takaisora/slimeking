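; BP_BRock is a rock pickup actor that characters and stray slimes consume by touching its static mesh.
; On overlap, a sequence casts the other actor to each of four character Blueprints, resetting that character's abilities, adding rock score and setting its BRock ability flag.
; A BP_Stray_slime only receives the rock score.
; Every successful branch shares one ending that plays the slime predation sound and destroys the rock.
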(event `self.StaticMesh.OnComponentBeginOverlap`
  (params (OverlappedComponent :type "PrimitiveComponent Object Reference") (OtherActor :type "Actor Object Reference") (OtherComp :type "PrimitiveComponent Object Reference") (OtherBodyIndex :type Integer) (bFromSweep :type Boolean) (SweepResult :type "HitResult Structure (by ref)"))
  (bind (_asbp_character_02 _bsuccess) (cast `/Game/BluePrints/BP_Character/BP_Character_02` OtherActor :!pure true))
  (bind (_asbp_character _bsuccess_2) (cast `/Game/BluePrints/BP_Character/BP_Character` OtherActor :!pure true))
  (bind (_asbp_character_03 _bsuccess_3) (cast `/Game/BluePrints/BP_Character/BP_Character_03` OtherActor :!pure true))
  (bind (_asbp_character_04 _bsuccess_4) (cast `/Game/BluePrints/BP_Character/BP_Character_04` OtherActor :!pure true))
  (bind (_asbp_stray_slime _bsuccess_5) (cast `/Game/Cave_Enemy/Stray_Slime/BP_Stray_slime` OtherActor :!pure true))
  (`|ExecutionSequence`
    (:`then_0`
      (if _bsuccess_2
        (`/Game/BluePrints/BP_Character/BP_Character.AbilityRisset` _asbp_character)
        (`/Game/BluePrints/BP_Character/BP_Character.AddScoreRock` _asbp_character)
        (set `/Game/BluePrints/BP_Character/BP_Character.BRockAbility` true _asbp_character)
        (`GameplayStatics.PlaySound2D` "/Game/Sounds/slime_Predation.slime_Predation" 1.0 1.0 0.0 null null :!label _label)
        (`self.K2_DestroyActor`)))
    (:`then_1`
      (if _bsuccess
        (`/Game/BluePrints/BP_Character/BP_Character_02.AbilityRisset` _asbp_character_02)
        (`/Game/BluePrints/BP_Character/BP_Character_02.AddScoreRock` _asbp_character_02)
        (set `/Game/BluePrints/BP_Character/BP_Character_02.BRockAbility` true _asbp_character_02)
        (goto _label)))
    (:`then_2`
      (if _bsuccess_3
        (`/Game/BluePrints/BP_Character/BP_Character_03.AbilityRisset` _asbp_character_03)
        (`/Game/BluePrints/BP_Character/BP_Character_03.AddScoreRock` _asbp_character_03)
        (set `/Game/BluePrints/BP_Character/BP_Character_03.BRockAbility` true _asbp_character_03)
        (goto _label)))
    (:`then_3`
      (if _bsuccess_4
        (`/Game/BluePrints/BP_Character/BP_Character_04.AbilityRisset` _asbp_character_04)
        (`/Game/BluePrints/BP_Character/BP_Character_04.AddScoreRock` _asbp_character_04)
        (set `/Game/BluePrints/BP_Character/BP_Character_04.BRockAbility` true _asbp_character_04)
        (goto _label)))
    (:`then_4`
      (if _bsuccess_5
        (`/Game/Cave_Enemy/Stray_Slime/BP_Stray_slime.AddScoreRock` _asbp_stray_slime)
        (goto _label)))))

(fn `UserConstructionScript`
  (`parent.UserConstructionScript`))