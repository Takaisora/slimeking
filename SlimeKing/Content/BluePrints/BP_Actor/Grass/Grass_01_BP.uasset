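; Grass pickup actor that awards score to a living player character on touch and then destroys itself.
; Its Box overlap event runs a sequence of casts to four separate character Blueprints, BP_Character through BP_Character_04.
; Each branch skips characters flagged as Death, otherwise calls that character's AddScore, and all branches share one DestroyActor call.
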(event `self.Box.OnComponentBeginOverlap`
  (params (OverlappedComponent :type "PrimitiveComponent Object Reference") (OtherActor :type "Actor Object Reference") (OtherComp :type "PrimitiveComponent Object Reference") (OtherBodyIndex :type Integer) (bFromSweep :type Boolean) (SweepResult :type "HitResult Structure (by ref)"))
  (bind (_asbp_character_02 _bsuccess) (cast `/Game/BluePrints/BP_Character/BP_Character_02` OtherActor :!pure true))
  (bind (_asbp_character _bsuccess_2) (cast `/Game/BluePrints/BP_Character/BP_Character` OtherActor :!pure true))
  (bind (_asbp_character_03 _bsuccess_3) (cast `/Game/BluePrints/BP_Character/BP_Character_03` OtherActor :!pure true))
  (bind (_asbp_character_04 _bsuccess_4) (cast `/Game/BluePrints/BP_Character/BP_Character_04` OtherActor :!pure true))
  (`|ExecutionSequence`
    (:`then_0`
      (if _bsuccess_2
        (if (not (`/Game/BluePrints/BP_Character/BP_Character.Death` _asbp_character))
          (`/Game/BluePrints/BP_Character/BP_Character.AddScore` _asbp_character)
          (`self.K2_DestroyActor` :!label _label))))
    (:`then_1`
      (if _bsuccess
        (if (not (`/Game/BluePrints/BP_Character/BP_Character_02.Death` _asbp_character_02))
          (`/Game/BluePrints/BP_Character/BP_Character_02.AddScore` _asbp_character_02)
          (goto _label))))
    (:`then_2`
      (if _bsuccess_3
        (if (not (`/Game/BluePrints/BP_Character/BP_Character_03.Death` _asbp_character_03))
          (`/Game/BluePrints/BP_Character/BP_Character_03.AddScore` _asbp_character_03)
          (goto _label))))
    (:`then_3`
      (if _bsuccess_4
        (if (not (`/Game/BluePrints/BP_Character/BP_Character_04.Death` _asbp_character_04))
          (`/Game/BluePrints/BP_Character/BP_Character_04.AddScore` _asbp_character_04)
          (goto _label))))))

(fn `UserConstructionScript`)