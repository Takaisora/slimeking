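; Grass pickup actor that awards score when one of the playable or tutorial characters touches it, then destroys itself.
; Its StaticMesh begin-overlap runs a Sequence of casts, one for each of eight character Blueprint classes.
; The first two characters trigger dedicated GrassScore functions, the others call their own AddScore, and every successful branch feeds a shared DestroyActor.
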(event `self.StaticMesh.OnComponentBeginOverlap`
  (params (OverlappedComponent :type "PrimitiveComponent Object Reference") (OtherActor :type "Actor Object Reference") (OtherComp :type "PrimitiveComponent Object Reference") (OtherBodyIndex :type Integer) (bFromSweep :type Boolean) (SweepResult :type "HitResult Structure (by ref)"))
  (bind (_asbp_character_turtrial _bsuccess) (cast `/Game/BluePrints/BP_Character/Turtorial/BP_Character_turtrial` OtherActor :!pure true))
  (bind (_asbp_character_02_turtorial _bsuccess_2) (cast `/Game/BluePrints/BP_Character/Turtorial/BP_Character_02_Turtorial` OtherActor :!pure true))
  (bind (_asbp_character_03_turtorial _bsuccess_3) (cast `/Game/BluePrints/BP_Character/Turtorial/BP_Character_03_Turtorial` OtherActor :!pure true))
  (bind (_asbp_character_04_turtorial _bsuccess_4) (cast `/Game/BluePrints/BP_Character/Turtorial/BP_Character_04_Turtorial` OtherActor :!pure true))
  (bind (_asbp_character_03 _bsuccess_5) (cast `/Game/BluePrints/BP_Character/BP_Character_03` OtherActor :!pure true))
  (bind (_asbp_character_04 _bsuccess_6) (cast `/Game/BluePrints/BP_Character/BP_Character_04` OtherActor :!pure true))
  (`|ExecutionSequence`
    (:`then_0`
      (if (`.bSuccess` (cast `/Game/BluePrints/BP_Character/BP_Character` OtherActor :!pure true))
        (`self.GrassScore_BP_01_01`)
        (`self.K2_DestroyActor` :!label _label)))
    (:`then_1`
      (if (`.bSuccess` (cast `/Game/BluePrints/BP_Character/BP_Character_02` OtherActor :!pure true))
        (`self.GrassScore_BP_02_01`)
        (goto _label)))
    (:`then_2`
      (if _bsuccess_5
        (`/Game/BluePrints/BP_Character/BP_Character_03.AddScore` _asbp_character_03)
        (goto _label)))
    (:`then_3`
      (if _bsuccess_6
        (`/Game/BluePrints/BP_Character/BP_Character_04.AddScore` _asbp_character_04)
        (goto _label)))
    (:`then_4`
      (if _bsuccess
        (`/Game/BluePrints/BP_Character/Turtorial/BP_Character_turtrial.AddScore` _asbp_character_turtrial)
        (goto _label)))
    (:`then_5`
      (if _bsuccess_2
        (`/Game/BluePrints/BP_Character/Turtorial/BP_Character_02_Turtorial.AddScore` _asbp_character_02_turtorial)
        (goto _label)))
    (:`then_6`
      (if _bsuccess_3
        (`/Game/BluePrints/BP_Character/Turtorial/BP_Character_03_Turtorial.AddScore` _asbp_character_03_turtorial)
        (goto _label)))
    (:`then_7`
      (if _bsuccess_4
        (`/Game/BluePrints/BP_Character/Turtorial/BP_Character_04_Turtorial.AddScore` _asbp_character_04_turtorial)
        (goto _label)))))

(fn `UserConstructionScript`)