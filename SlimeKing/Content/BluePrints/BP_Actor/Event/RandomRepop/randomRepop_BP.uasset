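; Random respawner actor that keeps populating the level with wolves, whisps, wing rabbits and lizards.
; From BeginPlay, Start_Pop spawns two of each immediately and re-sets a looping timer on itself to repeat every ten seconds, without any population cap.
; These spawns use random points in a fixed box around world origin and get default controllers.
; Salamander and Grass spawners use variable-defined areas and classes, but SetSpawn never calls them.
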(event `self.ReceiveBeginPlay`
  (`self.Start_Pop`))

(event `Start_Pop`
  (`KismetSystemLibrary.K2_SetTimerDelegate` (delegate `Start_Pop`) 10.0 true)
  (`self.Set_Spawn`))

(event `self.ReceiveTick`
  (params (DeltaSeconds :type "Float (single-precision)")))

(fn `Set_Spawn`
  (`self.Spawn_wolf`)
  (`self.Spawn_whisp`)
  (`self.Spawn_wingRabbit`)
  (`self.Spawn_lizard`)
  (`self.Spawn_wolf`)
  (`self.Spawn_whisp`)
  (`self.Spawn_wingRabbit`)
  (`self.Spawn_lizard`))

(fn `Spawn_lizard`
  (bind _returnvalue (`|SpawnActorFromClass` "/Game/Enemy/Lizard/BP_Lizard.BP_Lizard_C" (`KismetMathLibrary.Conv_VectorToTransform` (`KismetMathLibrary.RandomPointInBoundingBox` (0.0 0.0 0.0) (5000.0 5000.0 500.0))) "AlwaysSpawn" "OverrideRootScale" null null))
  (`Pawn.SpawnDefaultController` _returnvalue))

(fn `Spawn_salamander`
  (bind (_enemy _spawnarea_start _spawnarea_end) (break `/Game/BluePrints/BP_Actor/Event/RandomRepop/EnemySpawn` (`self.salamander`)))
  (bind _returnvalue (`|SpawnActorFromClass` _enemy (`KismetMathLibrary.MakeTransform` (`KismetMathLibrary.MakeVector` (`KismetMathLibrary.RandomFloatInRange` (.x _spawnarea_start) (.x _spawnarea_end)) (`KismetMathLibrary.RandomFloatInRange` (.y _spawnarea_start) (.y _spawnarea_end)) (`KismetMathLibrary.RandomFloatInRange` (.z _spawnarea_start) (.z _spawnarea_end))) (struct) (`self.spawnScale`)) "AlwaysSpawn" "OverrideRootScale" null null))
  (`Pawn.SpawnDefaultController` _returnvalue))

(fn `Spawn_whisp`
  (bind _returnvalue (`|SpawnActorFromClass` "/Game/Enemy/Whisp/BP_Whisp.BP_Whisp_C" (`KismetMathLibrary.Conv_VectorToTransform` (`KismetMathLibrary.RandomPointInBoundingBox` (0.0 0.0 0.0) (5000.0 5000.0 500.0))) "AlwaysSpawn" "OverrideRootScale" null null))
  (`Pawn.SpawnDefaultController` _returnvalue))

(fn `Spawn_wingRabbit`
  (bind _returnvalue (`|SpawnActorFromClass` "/Game/Enemy/WingRabbit/BP_WingRabbit.BP_WingRabbit_C" (`KismetMathLibrary.Conv_VectorToTransform` (`KismetMathLibrary.RandomPointInBoundingBox` (0.0 0.0 0.0) (5000.0 5000.0 500.0))) "AlwaysSpawn" "OverrideRootScale" null null))
  (`Pawn.SpawnDefaultController` _returnvalue))

(fn `Spawn_wolf`
  (bind _returnvalue (`|SpawnActorFromClass` "/Game/Enemy/Wolf/BP_Wolf.BP_Wolf_C" (`KismetMathLibrary.Conv_VectorToTransform` (`KismetMathLibrary.RandomPointInBoundingBox` (0.0 0.0 0.0) (5000.0 5000.0 500.0))) "AlwaysSpawn" "OverrideRootScale" null null))
  (`Pawn.SpawnDefaultController` _returnvalue))

(fn `SpawnGrass`
  (bind (_enemy _spawnarea_start _spawnarea_end) (break `/Game/BluePrints/BP_Actor/Event/RandomRepop/EnemySpawn` (`self.Grass`)))
  (bind _returnvalue (`|SpawnActorFromClass` _enemy (`KismetMathLibrary.MakeTransform` (`KismetMathLibrary.MakeVector` (`KismetMathLibrary.RandomFloatInRange` (.x _spawnarea_start) (.x _spawnarea_end)) (`KismetMathLibrary.RandomFloatInRange` (.y _spawnarea_start) (.y _spawnarea_end)) (`KismetMathLibrary.RandomFloatInRange` (.z _spawnarea_start) (.z _spawnarea_end))) (struct) (`self.spawnScale`)) "AlwaysSpawn" "OverrideRootScale" null null))
  (`Pawn.SpawnDefaultController` _returnvalue))

(fn `UserConstructionScript`)