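; Cave game mode, apparently for four players, that populates the level with creatures over time.
; BeginPlay starts a looping timer that periodically runs SetSpawn, and separately spawns one metal lizard at a fixed point after a delay.
; SetSpawn repeatedly calls helpers that place stray slimes, Koumori and HikariDake at random points in three boxes, each with a default controller.
; SpawnLizerd follows the same pattern but is never called here; AmeTime is empty.
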(event `self.ReceiveBeginPlay`
  (`|ExecutionSequence`
    (:`then_0`
      (`self.Start_Pop`))
    (:`then_1`
      (`KismetSystemLibrary.Delay` 104.0)
      (bind _returnvalue (`|SpawnActorFromClass` "/Game/Enemy/MetalLizard/testMetalLizard_BP.testMetalLizard_BP_C" (`KismetMathLibrary.MakeTransform` (-1200.0 1115.0 20.0) (struct :`Yaw` -20.0)) "Undefined" "OverrideRootScale" null null))
      (`Pawn.SpawnDefaultController` _returnvalue))))

(event `Start_Pop`
  (`KismetSystemLibrary.K2_SetTimerDelegate` (delegate `Start_Pop`) 50.0 true)
  (`self.Set_spawn`))

(fn `ameTime`)

(fn `Kouori`
  (`|ExecutionSequence`
    (:`then_0`
      (bind _returnvalue (`|SpawnActorFromClass` "/Game/Enemy/Koumori/Koumori_BP.Koumori_BP_C" (`KismetMathLibrary.Conv_VectorToTransform` (`KismetMathLibrary.RandomPointInBoundingBox` (-2873.0 -1400.0 600.0) (-5612.0 1300.0 500.0))) "AlwaysSpawn" "OverrideRootScale" null null))
      (`Pawn.SpawnDefaultController` _returnvalue))
    (:`then_1`
      (bind _returnvalue_2 (`|SpawnActorFromClass` "/Game/Enemy/Koumori/Koumori_BP.Koumori_BP_C" (`KismetMathLibrary.Conv_VectorToTransform` (`KismetMathLibrary.RandomPointInBoundingBox` (2800.0 -1500.0 600.0) (5880.0 1500.0 500.0))) "AlwaysSpawn" "OverrideRootScale" null null))
      (`Pawn.SpawnDefaultController` _returnvalue_2))
    (:`then_2`
      (bind _returnvalue_3 (`|SpawnActorFromClass` "/Game/Enemy/Koumori/Koumori_BP.Koumori_BP_C" (`KismetMathLibrary.Conv_VectorToTransform` (`KismetMathLibrary.RandomPointInBoundingBox` (2150.0 2150.0 50.0) (-2150.0 -2150.0 50.0))) "AlwaysSpawn" "OverrideRootScale" null null))
      (`Pawn.SpawnDefaultController` _returnvalue_3))))

(fn `Set_spawn`
  (`self.Spawn_caveslime`)
  (`self.Spawn_caveslime`)
  (`self.Spawn_caveslime`)
  (`self.Spawn_caveslime`)
  (`self.Kouori`)
  (`self.Kouori`)
  (`self.SpawnHikaridake`)
  (`self.SpawnHikaridake`))

(fn `Spawn_caveslime`
  (`|ExecutionSequence`
    (:`then_0`
      (bind _returnvalue (`|SpawnActorFromClass` "/Game/Cave_Enemy/Stray_Slime/BP_Stray_slime.BP_Stray_slime_C" (`KismetMathLibrary.Conv_VectorToTransform` (`KismetMathLibrary.RandomPointInBoundingBox` (-2873.0 -1400.0 600.0) (-5612.0 1300.0 500.0))) "AlwaysSpawn" "OverrideRootScale" null null))
      (`Pawn.SpawnDefaultController` _returnvalue))
    (:`then_1`
      (bind _returnvalue_2 (`|SpawnActorFromClass` "/Game/Cave_Enemy/Stray_Slime/BP_Stray_slime.BP_Stray_slime_C" (`KismetMathLibrary.Conv_VectorToTransform` (`KismetMathLibrary.RandomPointInBoundingBox` (2800.0 -1500.0 600.0) (5880.0 1500.0 500.0))) "AlwaysSpawn" "OverrideRootScale" null null))
      (`Pawn.SpawnDefaultController` _returnvalue_2))
    (:`then_2`
      (bind _returnvalue_3 (`|SpawnActorFromClass` "/Game/Cave_Enemy/Stray_Slime/BP_Stray_slime.BP_Stray_slime_C" (`KismetMathLibrary.Conv_VectorToTransform` (`KismetMathLibrary.RandomPointInBoundingBox` (2150.0 2150.0 0.0) (-2150.0 -2150.0 0.0))) "AlwaysSpawn" "OverrideRootScale" null null))
      (`Pawn.SpawnDefaultController` _returnvalue_3))))

(fn `Spawn_lizerd`
  (`|ExecutionSequence`
    (:`then_0`
      (bind _returnvalue (`|SpawnActorFromClass` "/Game/Enemy/MetalLizard/testMetalLizard_BP.testMetalLizard_BP_C" (`KismetMathLibrary.Conv_VectorToTransform` (`KismetMathLibrary.RandomPointInBoundingBox` (-2873.0 -1400.0 600.0) (-5612.0 1300.0 500.0))) "AlwaysSpawn" "OverrideRootScale" null null))
      (`Pawn.SpawnDefaultController` _returnvalue))
    (:`then_1`
      (bind _returnvalue_2 (`|SpawnActorFromClass` "/Game/Enemy/MetalLizard/testMetalLizard_BP.testMetalLizard_BP_C" (`KismetMathLibrary.Conv_VectorToTransform` (`KismetMathLibrary.RandomPointInBoundingBox` (2800.0 -1500.0 600.0) (5880.0 1500.0 500.0))) "AlwaysSpawn" "OverrideRootScale" null null))
      (`Pawn.SpawnDefaultController` _returnvalue_2))
    (:`then_2`
      (bind _returnvalue_3 (`|SpawnActorFromClass` "/Game/Enemy/MetalLizard/testMetalLizard_BP.testMetalLizard_BP_C" (`KismetMathLibrary.Conv_VectorToTransform` (`KismetMathLibrary.RandomPointInBoundingBox` (2150.0 2150.0 0.0) (-2150.0 -2150.0 0.0))) "AlwaysSpawn" "OverrideRootScale" null null))
      (`Pawn.SpawnDefaultController` _returnvalue_3))))

(fn `SpawnHikaridake`
  (`|ExecutionSequence`
    (:`then_0`
      (bind _returnvalue (`|SpawnActorFromClass` "/Game/Enemy/HikariDake/HikariDakeBP.HikariDakeBP_C" (`KismetMathLibrary.Conv_VectorToTransform` (`KismetMathLibrary.RandomPointInBoundingBox` (-2873.0 -1400.0 600.0) (-5612.0 1300.0 500.0))) "AlwaysSpawn" "OverrideRootScale" null null))
      (`Pawn.SpawnDefaultController` _returnvalue))
    (:`then_1`
      (bind _returnvalue_2 (`|SpawnActorFromClass` "/Game/Enemy/HikariDake/HikariDakeBP.HikariDakeBP_C" (`KismetMathLibrary.Conv_VectorToTransform` (`KismetMathLibrary.RandomPointInBoundingBox` (2800.0 -1500.0 600.0) (5880.0 1500.0 500.0))) "AlwaysSpawn" "OverrideRootScale" null null))
      (`Pawn.SpawnDefaultController` _returnvalue_2))
    (:`then_2`
      (bind _returnvalue_3 (`|SpawnActorFromClass` "/Game/Enemy/HikariDake/HikariDakeBP.HikariDakeBP_C" (`KismetMathLibrary.Conv_VectorToTransform` (`KismetMathLibrary.RandomPointInBoundingBox` (2150.0 2150.0 0.0) (-2150.0 -2150.0 0.0))) "AlwaysSpawn" "OverrideRootScale" null null))
      (`Pawn.SpawnDefaultController` _returnvalue_3))))

(fn `UserConstructionScript`)