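; Game mode, named for four players, that periodically populates the level with creatures.
; From BeginPlay, Start_Pop arms a looping timer on itself and calls Set_spawn, adding five each of wolves, winged rabbits and lizards per wave.
; Spawn helpers place them at random points in a fixed box, each with a default controller.
; The whisp spawner is never called, and local player creation and removal logic is disconnected.
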(event `self.ReceiveBeginPlay`
  (`self.Start_Pop`))

(event `Start_Pop`
  (`KismetSystemLibrary.K2_SetTimerDelegate` (delegate `Start_Pop`) 50.0 true)
  (`self.Set_spawn`))

(fn `ameTime`)

(fn `Set_spawn`
  (`self.Spawn_wolf`)
  (`self.Spawn_wingRabbit`)
  (`self.Spawn_lizard`)
  (`self.Spawn_wolf`)
  (`self.Spawn_wingRabbit`)
  (`self.Spawn_lizard`)
  (`self.Spawn_wolf`)
  (`self.Spawn_wingRabbit`)
  (`self.Spawn_lizard`)
  (`self.Spawn_wolf`)
  (`self.Spawn_wingRabbit`)
  (`self.Spawn_lizard`)
  (`self.Spawn_wolf`)
  (`self.Spawn_wingRabbit`)
  (`self.Spawn_lizard`))

(fn `Spawn_lizard`
  (bind _returnvalue (`|SpawnActorFromClass` "/Game/Enemy/Lizard/BP_Lizard.BP_Lizard_C" (`KismetMathLibrary.Conv_VectorToTransform` (`KismetMathLibrary.RandomPointInBoundingBox` (0.0 0.0 300.0) (5000.0 5000.0 500.0))) "AlwaysSpawn" "OverrideRootScale" null null))
  (`Pawn.SpawnDefaultController` _returnvalue))

(fn `Spawn_whisp`
  (bind _returnvalue (`|SpawnActorFromClass` "/Game/Enemy/Whisp/BP_Whisp.BP_Whisp_C" (`KismetMathLibrary.Conv_VectorToTransform` (`KismetMathLibrary.RandomPointInBoundingBox` (0.0 0.0 0.0) (5000.0 5000.0 500.0))) "AlwaysSpawn" "OverrideRootScale" null null))
  (`Pawn.SpawnDefaultController` _returnvalue))

(fn `Spawn_wingRabbit`
  (bind _returnvalue (`|SpawnActorFromClass` "/Game/Enemy/WingRabbit/BP_WingRabbit.BP_WingRabbit_C" (`KismetMathLibrary.Conv_VectorToTransform` (`KismetMathLibrary.RandomPointInBoundingBox` (0.0 0.0 300.0) (5000.0 5000.0 500.0))) "AlwaysSpawn" "OverrideRootScale" null null))
  (`Pawn.SpawnDefaultController` _returnvalue))

(fn `Spawn_wolf`
  (bind _returnvalue (`|SpawnActorFromClass` "/Game/Enemy/Wolf/BP_Wolf.BP_Wolf_C" (`KismetMathLibrary.Conv_VectorToTransform` (`KismetMathLibrary.RandomPointInBoundingBox` (0.0 0.0 300.0) (5000.0 5000.0 500.0))) "AlwaysSpawn" "OverrideRootScale" null null))
  (`Pawn.SpawnDefaultController` _returnvalue))

(fn `UserConstructionScript`)