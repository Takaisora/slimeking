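; Player controller with keyboard shortcuts that adjust the scores of all four slime players at once, apparently for testing.
; H adds ten and G subtracts ten from the Score on each of the four player characters, each cast to its own Blueprint class.
; Each new score is then copied into the matching slime score variable on GameInstace_BP.
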(event `Key|H`
  (params (Key :type "Key Structure"))
  (bind _asbp_character_04 (cast `/Game/BluePrints/BP_Character/BP_Character_04` (`GameplayStatics.GetPlayerCharacter` 3) :!pure true))
  (bind _asbp_character (cast `/Game/BluePrints/BP_Character/BP_Character` (`GameplayStatics.GetPlayerCharacter` 0) :!pure true))
  (bind _asbp_character_03 (cast `/Game/BluePrints/BP_Character/BP_Character_03` (`GameplayStatics.GetPlayerCharacter` 2) :!pure true))
  (bind _asbp_character_02 (cast `/Game/BluePrints/BP_Character/BP_Character_02` (`GameplayStatics.GetPlayerCharacter` 1) :!pure true))
  (:`Pressed`
    (`|ExecutionSequence`
      (:`then_0`
        (bind _output_get (set `/Game/BluePrints/BP_Character/BP_Character_04.Score` (+ (`/Game/BluePrints/BP_Character/BP_Character_04.Score` _asbp_character_04) 10) _asbp_character_04))
        (bind _asgame_instace_bp (cast `/Game/BluePrints/BP_Instance/GameInstace_BP` (`GameplayStatics.GetGameInstance`)))
        (set `/Game/BluePrints/BP_Instance/GameInstace_BP.slime_4_score` _output_get _asgame_instace_bp))
      (:`then_1`
        (bind _output_get_2 (set `/Game/BluePrints/BP_Character/BP_Character_03.Score` (+ (`/Game/BluePrints/BP_Character/BP_Character_03.Score` _asbp_character_03) 10) _asbp_character_03))
        (bind _asgame_instace_bp_2 (cast `/Game/BluePrints/BP_Instance/GameInstace_BP` (`GameplayStatics.GetGameInstance`)))
        (set `/Game/BluePrints/BP_Instance/GameInstace_BP.slime_3_score` _output_get_2 _asgame_instace_bp_2))
      (:`then_2`
        (bind _output_get_3 (set `/Game/BluePrints/BP_Character/BP_Character_02.Score` (+ (`/Game/BluePrints/BP_Character/BP_Character_02.Score` _asbp_character_02) 10) _asbp_character_02))
        (bind _asgame_instace_bp_3 (cast `/Game/BluePrints/BP_Instance/GameInstace_BP` (`GameplayStatics.GetGameInstance`)))
        (set `/Game/BluePrints/BP_Instance/GameInstace_BP.slime_2_score` _output_get_3 _asgame_instace_bp_3))
      (:`then_3`
        (bind _output_get_4 (set `/Game/BluePrints/BP_Character/BP_Character.Score` (+ (`/Game/BluePrints/BP_Character/BP_Character.Score` _asbp_character) 10) _asbp_character))
        (bind _asgame_instace_bp_4 (cast `/Game/BluePrints/BP_Instance/GameInstace_BP` (`GameplayStatics.GetGameInstance`)))
        (set `/Game/BluePrints/BP_Instance/GameInstace_BP.slime_1_score` _output_get_4 _asgame_instace_bp_4)))))

(event `Key|G`
  (params (Key :type "Key Structure"))
  (bind _asbp_character_04 (cast `/Game/BluePrints/BP_Character/BP_Character_04` (`GameplayStatics.GetPlayerCharacter` 3) :!pure true))
  (bind _asbp_character (cast `/Game/BluePrints/BP_Character/BP_Character` (`GameplayStatics.GetPlayerCharacter` 0) :!pure true))
  (bind _asbp_character_03 (cast `/Game/BluePrints/BP_Character/BP_Character_03` (`GameplayStatics.GetPlayerCharacter` 2) :!pure true))
  (bind _asbp_character_02 (cast `/Game/BluePrints/BP_Character/BP_Character_02` (`GameplayStatics.GetPlayerCharacter` 1) :!pure true))
  (:`Pressed`
    (`|ExecutionSequence`
      (:`then_0`
        (bind _output_get (set `/Game/BluePrints/BP_Character/BP_Character_04.Score` (+ (`/Game/BluePrints/BP_Character/BP_Character_04.Score` _asbp_character_04) -10) _asbp_character_04))
        (bind _asgame_instace_bp (cast `/Game/BluePrints/BP_Instance/GameInstace_BP` (`GameplayStatics.GetGameInstance`)))
        (set `/Game/BluePrints/BP_Instance/GameInstace_BP.slime_4_score` _output_get _asgame_instace_bp))
      (:`then_1`
        (bind _output_get_2 (set `/Game/BluePrints/BP_Character/BP_Character_03.Score` (+ (`/Game/BluePrints/BP_Character/BP_Character_03.Score` _asbp_character_03) -10) _asbp_character_03))
        (bind _asgame_instace_bp_2 (cast `/Game/BluePrints/BP_Instance/GameInstace_BP` (`GameplayStatics.GetGameInstance`)))
        (set `/Game/BluePrints/BP_Instance/GameInstace_BP.slime_3_score` _output_get_2 _asgame_instace_bp_2))
      (:`then_2`
        (bind _output_get_3 (set `/Game/BluePrints/BP_Character/BP_Character_02.Score` (+ (`/Game/BluePrints/BP_Character/BP_Character_02.Score` _asbp_character_02) -10) _asbp_character_02))
        (bind _asgame_instace_bp_3 (cast `/Game/BluePrints/BP_Instance/GameInstace_BP` (`GameplayStatics.GetGameInstance`)))
        (set `/Game/BluePrints/BP_Instance/GameInstace_BP.slime_2_score` _output_get_3 _asgame_instace_bp_3))
      (:`then_3`
        (bind _output_get_4 (set `/Game/BluePrints/BP_Character/BP_Character.Score` (+ (`/Game/BluePrints/BP_Character/BP_Character.Score` _asbp_character) -10) _asbp_character))
        (bind _asgame_instace_bp_4 (cast `/Game/BluePrints/BP_Instance/GameInstace_BP` (`GameplayStatics.GetGameInstance`)))
        (set `/Game/BluePrints/BP_Instance/GameInstace_BP.slime_1_score` _output_get_4 _asgame_instace_bp_4)))))

(fn `UserConstructionScript`)