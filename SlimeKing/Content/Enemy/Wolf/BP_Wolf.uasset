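; Wolf enemy that either gets absorbed by, or damages, one of four player slime characters based on score.
; PawnSensing writes any seen player character to the Blackboard "Player" key for its AI.
; On Box overlap, a character meeting its wolf threshold resets abilities, gains wolf score and ability, and destroys the wolf.
; Otherwise, characters scoring above 10 lose WolfAttack points, saved to their GameInstance slime score.
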(event `self.PawnSensing.OnSeePawn`
  (params (Pawn :type "Pawn Object Reference"))
  (bind _returnvalue (`AIBlueprintHelperLibrary.GetBlackboard` self))
  (`|ExecutionSequence`
    (:`then_0`
      (bind _asbp_character (cast `/Game/BluePrints/BP_Character/BP_Character` Pawn))
      (`BlackboardComponent.SetValueAsObject` _returnvalue "Player" _asbp_character))
    (:`then_1`
      (bind _asbp_character_02 (cast `/Game/BluePrints/BP_Character/BP_Character_02` Pawn))
      (`BlackboardComponent.SetValueAsObject` _returnvalue "Player" _asbp_character_02))
    (:`then_2`
      (bind _asbp_character_03 (cast `/Game/BluePrints/BP_Character/BP_Character_03` Pawn))
      (`BlackboardComponent.SetValueAsObject` _returnvalue "Player" _asbp_character_03))
    (:`then_3`
      (bind _asbp_character_04 (cast `/Game/BluePrints/BP_Character/BP_Character_04` Pawn))
      (`BlackboardComponent.SetValueAsObject` _returnvalue "Player" _asbp_character_04))))

(event `self.Box.OnComponentBeginOverlap`
  (params (OverlappedComponent :type "PrimitiveComponent Object Reference") (OtherActor :type "Actor Object Reference") (OtherComp :type "PrimitiveComponent Object Reference") (OtherBodyIndex :type Integer) (bFromSweep :type Boolean) (SweepResult :type "HitResult Structure (by ref)"))
  (bind (_asbp_character_03 _bsuccess) (cast `/Game/BluePrints/BP_Character/BP_Character_03` OtherActor :!pure true))
  (bind (_asbp_character _bsuccess_2) (cast `/Game/BluePrints/BP_Character/BP_Character` OtherActor :!pure true))
  (bind (_asbp_character_02 _bsuccess_3) (cast `/Game/BluePrints/BP_Character/BP_Character_02` OtherActor :!pure true))
  (bind (_asbp_character_04 _bsuccess_4) (cast `/Game/BluePrints/BP_Character/BP_Character_04` OtherActor :!pure true))
  (bind _score (`/Game/BluePrints/BP_Character/BP_Character.Score` _asbp_character))
  (bind _score_2 (`/Game/BluePrints/BP_Character/BP_Character_02.Score` _asbp_character_02))
  (bind _score_wolf (`/Game/BluePrints/BP_Character/BP_Character_03.score_wolf` _asbp_character_03))
  (bind _score_wolf_2 (`/Game/BluePrints/BP_Character/BP_Character.score_wolf` _asbp_character))
  (bind _score_wolf_2 (`/Game/BluePrints/BP_Character/BP_Character_02.score_wolf_2` _asbp_character_02))
  (bind _score_3 (`/Game/BluePrints/BP_Character/BP_Character_04.Score` _asbp_character_04))
  (bind _score_wolf_3 (`/Game/BluePrints/BP_Character/BP_Character_04.score_wolf` _asbp_character_04))
  (bind _score_4 (`/Game/BluePrints/BP_Character/BP_Character_03.Score` _asbp_character_03))
  (`|ExecutionSequence`
    (:`then_0`
      (if _bsuccess_2
        (if (>= _score _score_wolf_2)
          (`/Game/BluePrints/BP_Character/BP_Character.AbilityRisset` _asbp_character)
          (`/Game/BluePrints/BP_Character/BP_Character.AddScore_Wolf` _asbp_character self)
          (set `/Game/BluePrints/BP_Character/BP_Character.WolfAbility` true _asbp_character)
          (`self.K2_DestroyActor` :!label _label)
          (elif (< _score _score_wolf_2)
            (if (> _score 10)
              (bind _output_get (set `/Game/BluePrints/BP_Character/BP_Character.Score` (- _score (`self.WolfAttack`)) _asbp_character))
              (bind _asgame_instace_bp (cast `/Game/BluePrints/BP_Instance/GameInstace_BP` (`GameplayStatics.GetGameInstance`)))
              (set `/Game/BluePrints/BP_Instance/GameInstace_BP.slime_1_score` _output_get _asgame_instace_bp))))))
    (:`then_1`
      (if _bsuccess_3
        (if (>= _score_2 _score_wolf_2)
          (`/Game/BluePrints/BP_Character/BP_Character_02.AbilityRisset` _asbp_character_02)
          (`/Game/BluePrints/BP_Character/BP_Character_02.AddScore_Wolf` _asbp_character_02 self)
          (set `/Game/BluePrints/BP_Character/BP_Character_02.WolfAbirity2` true _asbp_character_02)
          (goto _label)
          (elif (< _score_2 _score_wolf_2)
            (if (> _score_2 10)
              (bind _output_get_2 (set `/Game/BluePrints/BP_Character/BP_Character_02.Score` (- _score_2 (`self.WolfAttack`)) _asbp_character_02))
              (bind _asgame_instace_bp_2 (cast `/Game/BluePrints/BP_Instance/GameInstace_BP` (`GameplayStatics.GetGameInstance`)))
              (set `/Game/BluePrints/BP_Instance/GameInstace_BP.slime_2_score` _output_get_2 _asgame_instace_bp_2))))))
    (:`then_2`
      (if _bsuccess
        (if (>= _score_4 _score_wolf)
          (`/Game/BluePrints/BP_Character/BP_Character_03.AbilityRisset` _asbp_character_03)
          (`/Game/BluePrints/BP_Character/BP_Character_03.AddScore_Wolf` _asbp_character_03 self)
          (set `/Game/BluePrints/BP_Character/BP_Character_03.WolfAbility` true _asbp_character_03)
          (goto _label)
          (elif (< _score_4 _score_wolf)
            (if (> _score_4 10)
              (bind _output_get_3 (set `/Game/BluePrints/BP_Character/BP_Character_03.Score` (- _score_4 (`self.WolfAttack`)) _asbp_character_03))
              (bind _asgame_instace_bp_3 (cast `/Game/BluePrints/BP_Instance/GameInstace_BP` (`GameplayStatics.GetGameInstance`)))
              (set `/Game/BluePrints/BP_Instance/GameInstace_BP.slime_3_score` _output_get_3 _asgame_instace_bp_3))))))
    (:`then_3`
      (if _bsuccess_4
        (if (>= _score_3 _score_wolf_3)
          (`/Game/BluePrints/BP_Character/BP_Character_04.AbilityRisset` _asbp_character_04)
          (`/Game/BluePrints/BP_Character/BP_Character_04.AddScore_Wolf` _asbp_character_04 self)
          (set `/Game/BluePrints/BP_Character/BP_Character_04.WolfAbility` true _asbp_character_04)
          (goto _label)
          (elif (< _score_3 _score_wolf_3)
            (if (> _score_3 10)
              (bind _output_get_4 (set `/Game/BluePrints/BP_Character/BP_Character_04.Score` (- _score_3 (`self.WolfAttack`)) _asbp_character_04))
              (bind _asgame_instace_bp_4 (cast `/Game/BluePrints/BP_Instance/GameInstace_BP` (`GameplayStatics.GetGameInstance`)))
              (set `/Game/BluePrints/BP_Instance/GameInstace_BP.slime_4_score` _output_get_4 _asgame_instace_bp_4))))))))

(fn `UserConstructionScript`)