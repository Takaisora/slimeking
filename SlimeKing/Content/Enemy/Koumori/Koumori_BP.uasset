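; Koumori enemy actor that characters and stray slimes consume on contact once their score is high enough.
; Sphere overlap tries casts to BP_Character, its 02 to 04 variants and BP_Stray_slime in sequence.
; Each branch compares the toucher's Score against its ScoreWingRabbit threshold rather than a Koumori-specific one.
; On success it calls that toucher's AddScoreKoumori and destroys the Koumori.
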(event `self.Sphere.OnComponentBeginOverlap`
  (params (OverlappedComponent :type "PrimitiveComponent Object Reference") (OtherActor :type "Actor Object Reference") (OtherComp :type "PrimitiveComponent Object Reference") (OtherBodyIndex :type Integer) (bFromSweep :type Boolean) (SweepResult :type "HitResult Structure (by ref)"))
  (bind (_asbp_character _bsuccess) (cast `/Game/BluePrints/BP_Character/BP_Character` OtherActor :!pure true))
  (bind (_asbp_character_02 _bsuccess_2) (cast `/Game/BluePrints/BP_Character/BP_Character_02` OtherActor :!pure true))
  (bind (_asbp_stray_slime _bsuccess_3) (cast `/Game/Cave_Enemy/Stray_Slime/BP_Stray_slime` OtherActor :!pure true))
  (bind (_asbp_character_03 _bsuccess_4) (cast `/Game/BluePrints/BP_Character/BP_Character_03` OtherActor :!pure true))
  (bind (_asbp_character_04 _bsuccess_5) (cast `/Game/BluePrints/BP_Character/BP_Character_04` OtherActor :!pure true))
  (`|ExecutionSequence`
    (:`then_0`
      (if _bsuccess
        (if (>= (`/Game/BluePrints/BP_Character/BP_Character.Score` _asbp_character) (`/Game/BluePrints/BP_Character/BP_Character.ScoreWingRabbit` _asbp_character))
          (`/Game/BluePrints/BP_Character/BP_Character.AddScoreKoumori` _asbp_character self)
          (`self.K2_DestroyActor` :!label _label))))
    (:`then_1`
      (if _bsuccess_2
        (if (>= (`/Game/BluePrints/BP_Character/BP_Character_02.Score` _asbp_character_02) (`/Game/BluePrints/BP_Character/BP_Character_02.Score_WingRabbitt` _asbp_character_02))
          (`/Game/BluePrints/BP_Character/BP_Character_02.AddScoreKoumori` _asbp_character_02 self)
          (goto _label))))
    (:`then_2`
      (if _bsuccess_4
        (if (>= (`/Game/BluePrints/BP_Character/BP_Character_03.Score` _asbp_character_03) (`/Game/BluePrints/BP_Character/BP_Character_03.ScoreWingRabbit` _asbp_character_03))
          (`/Game/BluePrints/BP_Character/BP_Character_03.AddScoreKoumori` _asbp_character_03 self)
          (goto _label))))
    (:`then_3`
      (if _bsuccess_5
        (if (>= (`/Game/BluePrints/BP_Character/BP_Character_04.Score` _asbp_character_04) (`/Game/BluePrints/BP_Character/BP_Character_04.ScoreWingRabbit` _asbp_character_04))
          (`/Game/BluePrints/BP_Character/BP_Character_04.AddScoreKoumori` _asbp_character_04 self)
          (goto _label))))
    (:`then_4`
      (if _bsuccess_3
        (if (>= (`/Game/Cave_Enemy/Stray_Slime/BP_Stray_slime.Score` _asbp_stray_slime) (`/Game/Cave_Enemy/Stray_Slime/BP_Stray_slime.ScoreWingRabbit` _asbp_stray_slime))
          (`/Game/Cave_Enemy/Stray_Slime/BP_Stray_slime.AddScoreKoumori` _asbp_stray_slime)
          (goto _label))))))

(fn `UserConstructionScript`)