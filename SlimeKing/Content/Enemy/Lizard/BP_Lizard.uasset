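; BP_Lizard is a lizard actor that any of the four player character classes can consume for points once their score is high enough.
; A Box overlap checks each class in sequence, requiring the character to be alive with Score at or above its ScoreLizard value.
; A qualifying character receives AddScoreLizard, then the lizard destroys itself.
; Two helper functions that award players 0 and 1 directly are not called within this Blueprint.
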(event `self.ReceiveBeginPlay`)

(event `self.ReceiveTick`
  (params (DeltaSeconds :type "Float (single-precision)")))

(event `self.Box.OnComponentBeginOverlap`
  (params (OverlappedComponent :type "PrimitiveComponent Object Reference") (OtherActor :type "Actor Object Reference") (OtherComp :type "PrimitiveComponent Object Reference") (OtherBodyIndex :type Integer) (bFromSweep :type Boolean) (SweepResult :type "HitResult Structure (by ref)"))
  (bind (_asbp_character _bsuccess) (cast `/Game/BluePrints/BP_Character/BP_Character` OtherActor :!pure true))
  (bind (_asbp_character_02 _bsuccess_2) (cast `/Game/BluePrints/BP_Character/BP_Character_02` OtherActor :!pure true))
  (bind (_asbp_character_03 _bsuccess_3) (cast `/Game/BluePrints/BP_Character/BP_Character_03` OtherActor :!pure true))
  (bind (_asbp_character_04 _bsuccess_4) (cast `/Game/BluePrints/BP_Character/BP_Character_04` OtherActor :!pure true))
  (`|ExecutionSequence`
    (:`then_0`
      (if _bsuccess
        (if (`/Game/BluePrints/BP_Character/BP_Character.Death` _asbp_character)
          _
          (elif (>= (`/Game/BluePrints/BP_Character/BP_Character.Score` _asbp_character) (`/Game/BluePrints/BP_Character/BP_Character.ScoreLizard` _asbp_character))
            (`/Game/BluePrints/BP_Character/BP_Character.AddScoreLizard` _asbp_character self)
            (`self.K2_DestroyActor` :!label _label)))))
    (:`then_1`
      (if _bsuccess_2
        (if (`/Game/BluePrints/BP_Character/BP_Character_02.Death` _asbp_character_02)
          _
          (elif (>= (`/Game/BluePrints/BP_Character/BP_Character_02.Score` _asbp_character_02) (`/Game/BluePrints/BP_Character/BP_Character_02.ScoreLizard` _asbp_character_02))
            (`/Game/BluePrints/BP_Character/BP_Character_02.AddScoreLizard` _asbp_character_02 self)
            (goto _label)))))
    (:`then_2`
      (if _bsuccess_3
        (if (`/Game/BluePrints/BP_Character/BP_Character_03.Death` _asbp_character_03)
          _
          (elif (>= (`/Game/BluePrints/BP_Character/BP_Character_03.Score` _asbp_character_03) (`/Game/BluePrints/BP_Character/BP_Character_03.ScoreLizard` _asbp_character_03))
            (`/Game/BluePrints/BP_Character/BP_Character_03.AddScoreLizard` _asbp_character_03 self)
            (goto _label)))))
    (:`then_3`
      (if _bsuccess_4
        (if (`/Game/BluePrints/BP_Character/BP_Character_04.Death` _asbp_character_04)
          _
          (elif (>= (`/Game/BluePrints/BP_Character/BP_Character_04.Score` _asbp_character_04) (`/Game/BluePrints/BP_Character/BP_Character_04.ScoreLizard` _asbp_character_04))
            (`/Game/BluePrints/BP_Character/BP_Character_04.AddScoreLizard` _asbp_character_04 self)
            (goto _label)))))))

(event `self.StaticMesh.OnComponentBeginOverlap`
  (params (OverlappedComponent :type "PrimitiveComponent Object Reference") (OtherActor :type "Actor Object Reference") (OtherComp :type "PrimitiveComponent Object Reference") (OtherBodyIndex :type Integer) (bFromSweep :type Boolean) (SweepResult :type "HitResult Structure (by ref)")))

(fn `LizardScoreBP1`
  (bind _asbp_character (cast `/Game/BluePrints/BP_Character/BP_Character` (`GameplayStatics.GetPlayerCharacter` 0)))
  (`/Game/BluePrints/BP_Character/BP_Character.AddScoreLizard` _asbp_character null))

(fn `LizardScoreBP2`
  (bind _asbp_character_02 (cast `/Game/BluePrints/BP_Character/BP_Character_02` (`GameplayStatics.GetPlayerCharacter` 1)))
  (`/Game/BluePrints/BP_Character/BP_Character_02.AddScoreLizard` _asbp_character_02 null))

(fn `UserConstructionScript`)