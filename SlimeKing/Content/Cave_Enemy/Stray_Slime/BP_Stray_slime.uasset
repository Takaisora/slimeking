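; BP_Stray_slime is an AI-driven stray slime in the cave that bigger player slimes absorb.
; On sphere overlap, any of four player characters with a higher score gains its score, updates that GameInstance slot and destroys it.
; PawnSensing writes seen players and other stray slimes to the Blackboard.
; Player-style helpers for score-based mesh scaling, abilities, inventory and splitting are defined but not called here, many hardwired to player one.
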(event `self.ReceiveBeginPlay`
  (set `self.score_slime` 1)
  (set `self.ScoreHikaridake` 20)
  (set `self.ScoreHikaridake` 10)
  (set `self.ScoreRock` 5))

(event `self.Sphere.OnComponentBeginOverlap`
  (params (OverlappedComponent :type "PrimitiveComponent Object Reference") (OtherActor :type "Actor Object Reference") (OtherComp :type "PrimitiveComponent Object Reference") (OtherBodyIndex :type Integer) (bFromSweep :type Boolean) (SweepResult :type "HitResult Structure (by ref)"))
  (bind (_asbp_character_02 _bsuccess) (cast `/Game/BluePrints/BP_Character/BP_Character_02` OtherActor :!pure true))
  (bind (_asbp_character _bsuccess_2) (cast `/Game/BluePrints/BP_Character/BP_Character` OtherActor :!pure true))
  (bind (_asbp_character_04 _bsuccess_3) (cast `/Game/BluePrints/BP_Character/BP_Character_04` OtherActor :!pure true))
  (bind (_asbp_character_03 _bsuccess_4) (cast `/Game/BluePrints/BP_Character/BP_Character_03` OtherActor :!pure true))
  (bind _score (`self.Score`))
  (bind _asgame_instace_bp (cast `/Game/BluePrints/BP_Instance/GameInstace_BP` (`GameplayStatics.GetGameInstance`) :!pure true))
  (bind _score_2 (`/Game/BluePrints/BP_Character/BP_Character.Score` _asbp_character))
  (bind _score_3 (`/Game/BluePrints/BP_Character/BP_Character_02.Score` _asbp_character_02))
  (bind _score_4 (`/Game/BluePrints/BP_Character/BP_Character_03.Score` _asbp_character_03))
  (bind _score_5 (`/Game/BluePrints/BP_Character/BP_Character_04.Score` _asbp_character_04))
  (`|ExecutionSequence`
    (:`then_0`
      (if _bsuccess_2
        (if (< _score _score_2)
          (bind _output_get (set `/Game/BluePrints/BP_Character/BP_Character.Score` (+ _score_2 _score) _asbp_character))
          (set `/Game/BluePrints/BP_Instance/GameInstace_BP.slime_1_score` _output_get _asgame_instace_bp)
          (`self.K2_DestroyActor` :!label _label))))
    (:`then_1`
      (if _bsuccess
        (if (< _score _score_3)
          (bind _output_get_2 (set `/Game/BluePrints/BP_Character/BP_Character_02.Score` (+ _score_3 _score) _asbp_character_02))
          (set `/Game/BluePrints/BP_Instance/GameInstace_BP.slime_2_score` _output_get_2 _asgame_instace_bp)
          (goto _label))))
    (:`then_2`
      (if _bsuccess_4
        (if (< _score _score_4)
          (bind _output_get_3 (set `/Game/BluePrints/BP_Character/BP_Character_03.Score` (+ _score_4 _score) _asbp_character_03))
          (set `/Game/BluePrints/BP_Instance/GameInstace_BP.slime_3_score` _output_get_3 _asgame_instace_bp)
          (goto _label))))
    (:`then_3`
      (if _bsuccess_3
        (if (< _score _score_5)
          (bind _output_get_4 (set `/Game/BluePrints/BP_Character/BP_Character_04.Score` (+ _score_5 _score) _asbp_character_04))
          (set `/Game/BluePrints/BP_Instance/GameInstace_BP.slime_4_score` _output_get_4 _asgame_instace_bp)
          (goto _label))))))

(event `self.PawnSensing.OnSeePawn`
  (params (Pawn :type "Pawn Object Reference"))
  (bind _returnvalue (`AIBlueprintHelperLibrary.GetBlackboard` self))
  (`|ExecutionSequence`
    (:`then_0`
      (bind _asbp_stray_slime (cast `/Game/Cave_Enemy/Stray_Slime/BP_Stray_slime` Pawn))
      (`BlackboardComponent.SetValueAsObject` _returnvalue "Stray_slime" _asbp_stray_slime))
    (:`then_1`
      (bind _asbp_character (cast `/Game/BluePrints/BP_Character/BP_Character` Pawn))
      (`BlackboardComponent.SetValueAsObject` _returnvalue "Player" _asbp_character))
    (:`then_2`
      (bind _asbp_character_02 (cast `/Game/BluePrints/BP_Character/BP_Character_02` Pawn))
      (`BlackboardComponent.SetValueAsObject` _returnvalue "Player" _asbp_character_02))
    (:`then_3`
      (bind _asbp_character_03 (cast `/Game/BluePrints/BP_Character/BP_Character_03` Pawn))
      (`BlackboardComponent.SetValueAsObject` _returnvalue "Player" _asbp_character_03))
    (:`then_4`
      (bind _asbp_character_04 (cast `/Game/BluePrints/BP_Character/BP_Character_04` Pawn))
      (`BlackboardComponent.SetValueAsObject` _returnvalue "Player" _asbp_character_04))))

(fn `AbilityJumpStetas`
  (set `CharacterMovementComponent.JumpZVelocity` 800.0 (`self.CharacterMovement`)))

(fn `AbilityWalkSpeed`
  (set `CharacterMovementComponent.MaxWalkSpeed` 600.0 (`self.CharacterMovement`)))

(fn `AddItem`
  (bind _actortrace (`self.ActorTrace`))
  (bind _actortrace_2 (`self.ActorTrace`))
  (bind (_asbp_wolf _bsuccess) (cast `/Game/Enemy/Wolf/BP_Wolf` _actortrace :!pure true))
  (bind (_asbp_wing_rabbit _bsuccess_2) (cast `/Game/Enemy/WingRabbit/BP_WingRabbit` _actortrace :!pure true))
  (bind (_asbp_whisp _bsuccess_3) (cast `/Game/Enemy/Whisp/BP_Whisp` _actortrace :!pure true))
  (bind (_asbp_wing_rabbit_2 _bsuccess_4) (cast `/Game/Enemy/WingRabbit/BP_WingRabbit` _actortrace_2 :!pure true))
  (bind (_asbp_wolf_2 _bsuccess_5) (cast `/Game/Enemy/Wolf/BP_Wolf` _actortrace_2 :!pure true))
  (bind (_asbp_whisp_2 _bsuccess_6) (cast `/Game/Enemy/Whisp/BP_Whisp` _actortrace_2 :!pure true))
  (if (`self.HaveItem?`)
    (set `self.WispAbility` false)
    (set `self.WolfAbility` false)
    (set `self.WingRabitAbility` false)
    (`|ExecutionSequence`
      (:`then_0`
        (if _bsuccess
          (`KismetArrayLibrary.Array_Add` (`self.Inventory`) (`/Game/BluePrints/BP_Inventory/Inventory/test.ItemData` _asbp_wolf))
          (set `self.WolfAbility` true)
          (set `self.HaveItem?` true :!label _label)
          (return)))
      (:`then_1`
        (if _bsuccess_3
          (`KismetArrayLibrary.Array_Add` (`self.Inventory`) (`/Game/BluePrints/BP_Inventory/Inventory/test.ItemData` _asbp_whisp))
          (set `self.WispAbility` true)
          (goto _label)))
      (:`then_2`
        (if _bsuccess_2
          (`KismetArrayLibrary.Array_Add` (`self.Inventory`) (`/Game/BluePrints/BP_Inventory/Inventory/test.ItemData` _asbp_wing_rabbit))
          (set `self.WingRabitAbility` true)
          (goto _label))))
    (else
      (`|ExecutionSequence`
        (:`then_0`
          (if _bsuccess_5
            (`KismetArrayLibrary.Array_Add` (`self.Inventory`) (`/Game/BluePrints/BP_Inventory/Inventory/test.ItemData` _asbp_wolf_2))
            (set `self.WolfAbility` true)
            (set `self.HaveItem?` true :!label _label_2)
            (return)))
        (:`then_1`
          (if _bsuccess_6
            (`KismetArrayLibrary.Array_Add` (`self.Inventory`) (`/Game/BluePrints/BP_Inventory/Inventory/test.ItemData` _asbp_whisp_2))
            (set `self.WispAbility` true)
            (goto _label_2)))
        (:`then_2`
          (if _bsuccess_4
            (`KismetArrayLibrary.Array_Add` (`self.Inventory`) (`/Game/BluePrints/BP_Inventory/Inventory/test.ItemData` _asbp_wing_rabbit_2))
            (set `self.WingRabitAbility` true)
            (goto _label_2)))))))

(fn `AddScore`
  (bind _output_get (set `self.Score` (+ (`self.Score`) (`self.score_slime`))))
  (`SceneComponent.SetWorldScale3D` (`self.Mesh`) (+ (`self.magnification_vector`) (* (/ _output_get (`self.magnification_score`)) (`self.magnification`)))))

(fn `AddScore_Wolf`
  (bind _output_get (set `self.Score` (+ (`self.Score`) (`self.score_wolf`))))
  (`SceneComponent.SetWorldScale3D` (`self.Mesh`) (+ (`self.magnification_vector`) (* (/ _output_get (`self.magnification_score`)) (`self.magnification`))))
  (bind _asgame_instace_bp (cast `/Game/BluePrints/BP_Instance/GameInstace_BP` (`GameplayStatics.GetGameInstance`)))
  (set `/Game/BluePrints/BP_Instance/GameInstace_BP.slime_1_score` (`self.Score`) _asgame_instace_bp)
  (`GameplayStatics.PlaySoundAtLocation` "/Game/Sounds/03_Slime_Acquired.03_Slime_Acquired" (`self.K2_GetActorLocation` (`GameplayStatics.GetPlayerCharacter` 0)) (struct) 1.0 1.0 0.0 "/Game/Sounds/NewSoundAttenuation.NewSoundAttenuation" null null))

(fn `AddScoreHikaridake`
  (bind _output_get (set `self.Score` (+ (`self.Score`) (`self.ScoreHikaridake`))))
  (`SceneComponent.SetWorldScale3D` (`self.Mesh`) (+ (`self.magnification_vector`) (* (/ _output_get (`self.magnification_score`)) (`self.magnification`))))
  (bind _asgame_instace_bp (cast `/Game/BluePrints/BP_Instance/GameInstace_BP` (`GameplayStatics.GetGameInstance`)))
  (set `/Game/BluePrints/BP_Instance/GameInstace_BP.slime_1_score` (`self.Score`) _asgame_instace_bp)
  (`GameplayStatics.PlaySoundAtLocation` "/Game/Sounds/03_Slime_Acquired.03_Slime_Acquired" (`self.K2_GetActorLocation` (`GameplayStatics.GetPlayerCharacter` 0)) (struct) 1.0 1.0 0.0 "/Game/Sounds/NewSoundAttenuation.NewSoundAttenuation" null null))

(fn `AddScoreKoumori`
  (bind _output_get (set `self.Score` (+ (`self.Score`) (`self.ScoreWingRabbit`))))
  (`SceneComponent.SetWorldScale3D` (`self.Mesh`) (+ (`self.magnification_vector`) (* (/ _output_get (`self.magnification_score`)) (`self.magnification`))))
  (`GameplayStatics.PlaySoundAtLocation` "/Game/Sounds/03_Slime_Acquired.03_Slime_Acquired" (`self.K2_GetActorLocation` (`GameplayStatics.GetPlayerCharacter` 0)) (struct) 1.0 1.0 0.0 "/Game/Sounds/NewSoundAttenuation.NewSoundAttenuation" null null))

(fn `AddScoreLizard`
  (bind _output_get (set `self.Score` (+ (`self.Score`) (`self.ScoreLizard`))))
  (`SceneComponent.SetWorldScale3D` (`self.Mesh`) (+ (`self.magnification_vector`) (* (/ _output_get (`self.magnification_score`)) (`self.magnification`))))
  (bind _asgame_instace_bp (cast `/Game/BluePrints/BP_Instance/GameInstace_BP` (`GameplayStatics.GetGameInstance`)))
  (set `/Game/BluePrints/BP_Instance/GameInstace_BP.slime_1_score` (`self.Score`) _asgame_instace_bp))

(fn `AddScoreRock`
  (bind _output_get (set `self.Score` (+ (`self.Score`) (`self.ScoreRock`))))
  (`SceneComponent.SetWorldScale3D` (`self.Mesh`) (+ (`self.magnification_vector`) (* (/ _output_get (`self.magnification_score`)) (`self.magnification`)))))

(fn `AddScoreWingRabbit`
  (bind _output_get (set `self.Score` (+ (`self.Score`) (`self.ScoreWingRabbit`))))
  (`SceneComponent.SetWorldScale3D` (`self.Mesh`) (+ (`self.magnification_vector`) (* (/ _output_get (`self.magnification_score`)) (`self.magnification`))))
  (bind _asgame_instace_bp (cast `/Game/BluePrints/BP_Instance/GameInstace_BP` (`GameplayStatics.GetGameInstance`)))
  (set `/Game/BluePrints/BP_Instance/GameInstace_BP.slime_1_score` (`self.Score`) _asgame_instace_bp)
  (`GameplayStatics.PlaySoundAtLocation` "/Game/Sounds/03_Slime_Acquired.03_Slime_Acquired" (`self.K2_GetActorLocation` (`GameplayStatics.GetPlayerCharacter` 0)) (struct) 1.0 1.0 0.0 "/Game/Sounds/NewSoundAttenuation.NewSoundAttenuation" null null))

(fn `AddScoreWisp`
  (bind _output_get (set `self.Score` (+ (`self.Score`) (`self.ScoreWisp`))))
  (`SceneComponent.SetWorldScale3D` (`self.Mesh`) (+ (`self.magnification_vector`) (* (/ _output_get (`self.magnification_score`)) (`self.magnification`))))
  (bind _asgame_instace_bp (cast `/Game/BluePrints/BP_Instance/GameInstace_BP` (`GameplayStatics.GetGameInstance`)))
  (set `/Game/BluePrints/BP_Instance/GameInstace_BP.slime_1_score` (`self.Score`) _asgame_instace_bp)
  (`GameplayStatics.PlaySoundAtLocation` "/Game/Sounds/03_Slime_Acquired.03_Slime_Acquired" (`self.K2_GetActorLocation` (`GameplayStatics.GetPlayerCharacter` 0)) (struct) 1.0 1.0 0.0 "/Game/Sounds/NewSoundAttenuation.NewSoundAttenuation" null null))

(fn `JumpUseScore`
  (set `self.Score` (- (`self.Score`) (`self.JumpScore`))))

(fn `ScoreGameInstance`
  (bind _asgame_instace_bp (cast `/Game/BluePrints/BP_Instance/GameInstace_BP` (`GameplayStatics.GetGameInstance`)))
  (bind _output_get (set `/Game/BluePrints/BP_Instance/GameInstace_BP.slime_1_score` (`self.Score`) _asgame_instace_bp))
  (`KismetSystemLibrary.PrintText` (`KismetTextLibrary.Conv_IntToText` _output_get)))

(fn `ScoreInstance`
  (bind _asgame_instace_bp (cast `/Game/BluePrints/BP_Instance/GameInstace_BP` (`GameplayStatics.GetGameInstance`)))
  (set `/Game/BluePrints/BP_Instance/GameInstace_BP.slime_1_score` (`self.Score`) _asgame_instace_bp))

(fn `SetWingRabbit`
  (set `CharacterMovementComponent.JumpZVelocity` 1600.0 (`self.CharacterMovement`))
  (`self.Jump` (`GameplayStatics.GetPlayerCharacter` 0)))

(fn `SetWisp`
  (`GameplayStatics.SpawnEmitterAtLocation` "/Game/Perticle/WhispParticle1.WhispParticle1" (`SceneComponent.K2_GetComponentLocation` (`/Game/BluePrints/BP_Character/BP_Character_02.Camera` (cast `/Game/BluePrints/BP_Character/BP_Character_02` (`GameplayStatics.GetPlayerCharacter` 1) :!pure true)))))

(fn `SetWolf`
  (set `CharacterMovementComponent.MaxWalkSpeed` (`self.speed`) (`self.CharacterMovement`))
  (return))

(fn `SplitSlime`
  (bind _returnvalue (`|SpawnActorFromClass` "/Game/BluePrints/BP_Character/AI/BP_Character_Child.BP_Character_Child_C" (`KismetMathLibrary.MakeTransform` (`KismetMathLibrary.RandomPointInBoundingBox` (`SceneComponent.K2_GetComponentLocation` (`self.Mesh`)) (`KismetMathLibrary.MakeVector` (`KismetMathLibrary.RandomFloatInRange` 500.0 500.0) (`KismetMathLibrary.RandomFloatInRange` -500.0 500.0)))) "Undefined" "OverrideRootScale" null null))
  (`self.SpawnDefaultController` _returnvalue))

(fn `UserConstructionScript`)

(fn `WingRabbitSound`
  (`GameplayStatics.PlaySoundAtLocation` "/Game/Sounds/14_SlimeWing_Descent.14_SlimeWing_Descent" (`self.K2_GetActorLocation` (`GameplayStatics.GetPlayerCharacter` 0)) (struct) 1.0 1.0 0.0 null null null) ; SlimeWing_Descent
)